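; BP_AmmoPickup is a purchasable ammo point in the horde mode where the player spends points to resupply ammo.
; Overlap with the first-person character stores a player reference and shows the cost through the horde game mode; any actor leaving hides it.
; While overlapping, the Use input has the game mode check and deduct points, then adds ammo to the player and refreshes the ammo UI.
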(event `EnhancedInput|/Game/FirstPerson/Input/Actions/IA_Use`
  (params (ActionValue :type Boolean) (ElapsedSeconds :type "Float (double-precision)") (TriggeredSeconds :type "Float (double-precision)") (InputAction :type "InputAction Object Reference" :default "/Game/FirstPerson/Input/Actions/IA_Use.IA_Use"))
  (bind _playerref (`self.PlayerRef`))
  (bind _ui_widget (`/Game/FirstPerson/Blueprints/BP_FirstPersonCharacter.UI Widget` _playerref))
  (:`Triggered`
    (if (`self.Overlapping`)
      (bind _asbp_horde_game_mode (cast `/Game/HordeCore/Blueprints/Game/BP_HordeGameMode` (`GameplayStatics.GetGameMode`)))
      (bind _result (`/Game/HordeCore/Blueprints/Game/BP_HordeGameMode.CanAfford` _asbp_horde_game_mode (`self.Points Value`)))
      (if _result
        (`/Game/HordeCore/Blueprints/Game/BP_HordeGameMode.SpendPoints` _asbp_horde_game_mode (`self.Points Value`))
        (`/Game/FirstPerson/Blueprints/BP_FirstPersonCharacter.Add Ammo` _playerref (`self.AmountToSupply`))
        (`/Game/HordeCore/Widgets/WBP_HUD.Update_CurrentAmmo_Text` _ui_widget)
        (`/Game/HordeCore/Widgets/WBP_HUD.Update_Reserve_Ammo_Text` _ui_widget)))))

(event `self.ReceiveActorEndOverlap`
  (params (OtherActor :type "Actor Object Reference"))
  (bind _asbp_horde_game_mode (cast `/Game/HordeCore/Blueprints/Game/BP_HordeGameMode` (`GameplayStatics.GetGameMode`)))
  (`/Game/HordeCore/Blueprints/Game/BP_HordeGameMode.HideWeaponPurchaseInfo` _asbp_horde_game_mode)
  (set `self.Overlapping` false))

(event `self.ReceiveActorBeginOverlap`
  (params (OtherActor :type "Actor Object Reference"))
  (bind _asbp_first_person_character (cast `/Game/FirstPerson/Blueprints/BP_FirstPersonCharacter` OtherActor))
  (set `self.PlayerRef` _asbp_first_person_character)
  (bind _asbp_horde_game_mode (cast `/Game/HordeCore/Blueprints/Game/BP_HordeGameMode` (`GameplayStatics.GetGameMode`)))
  (`/Game/HordeCore/Blueprints/Game/BP_HordeGameMode.ShowWeaponPurchaseInfo` _asbp_horde_game_mode (`self.Points Value`))
  (set `self.Overlapping` true))

(event `self.ReceiveBeginPlay`
  (`self.EnableInput` (`GameplayStatics.GetPlayerController` 0)))

(fn `UserConstructionScript`)