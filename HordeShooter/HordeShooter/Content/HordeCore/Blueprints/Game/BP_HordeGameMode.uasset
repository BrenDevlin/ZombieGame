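; Game mode for a horde survival game, running a warmup countdown, timed play and player death through a Tick-driven state.
; It owns the HUD and points economy: multiplied kill rewards, weapon purchase prompts, affordability checks and spending.
; BeginPlay async-loads or creates the save object that collects kill counts.
; On death it disables input and copies shot stats and survival time, writing to disk with the director's wave only on a best time.
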(event `PlayerKilled`
  (set `self.CurrentState` "NewEnumerator2")
  (`self.DisablePlayerInput`)
  (`self.SaveStats`))

(event `ZombieKilled`
  (params (PointsValue :type Integer))
  (bind _savedataobject (`self.SaveDataObject`))
  (set `self.CurrentPoints` (+ (* PointsValue (`self.PointsMultiplier`)) (`self.CurrentPoints`)))
  (`self.UpdatePointsDisplay`)
  (bind _result (`/Engine/EditorBlueprintResources/StandardMacros.IncrementInt` (`/Game/HordeCore/Blueprints/Game/BP_HordeGameSave.ZombieKills` _savedataobject))
    (:`  `
      (set `/Game/HordeCore/Blueprints/Game/BP_HordeGameSave.ZombieKills` _result _savedataobject))))

(event `self.ReceiveBeginPlay`
  (bind _returnvalue (`GameplayStatics.DoesSaveGameExist` "A"))
  (if _returnvalue
    (bind (_savegame _bsuccess) (`AsyncActionHandleSaveGame.AsyncLoadGameFromSlot` "A")
      (:`then`
        (`|ExecutionSequence` :!label _label
          (:`then_0`
            (bind _returnvalue_2 (`|CreateWidget` "/Game/HordeCore/Widgets/GameMode_HUD.GameMode_HUD_C"))
            (bind _output_get (set `self.GameModeHud` _returnvalue_2))
            (`UserWidget.AddToViewport` _output_get 0))
          (:`then_1`
            (`self.UpdatePointsDisplay`))
          (:`then_2`
            (`self.DisablePlayerInput`))
          (:`then_3`
            (`self.HideWeaponPurchaseInfo`))
          (:`then_4`
            (bind _returnvalue_3 (`GameplayStatics.GetActorOfClass` "/Game/HordeCore/Blueprints/Director/BP_Director.BP_Director_C"))
            (set `self.DirectorRef` _returnvalue_3))))
      (:`Completed`
        (if _bsuccess
          (bind _asbp_horde_game_save (cast `/Game/HordeCore/Blueprints/Game/BP_HordeGameSave` _savegame))
          (set `self.SaveDataObject` _asbp_horde_game_save))))
    (else
      (bind _returnvalue_4 (`GameplayStatics.CreateSaveGameObject` "/Game/HordeCore/Blueprints/Game/BP_HordeGameSave.BP_HordeGameSave_C"))
      (set `self.SaveDataObject` _returnvalue_4)
      (goto _label))))

(event `self.ReceiveTick`
  (params (DeltaSeconds :type "Float (single-precision)"))
  (switch `/Game/HordeCore/Blueprints/Game/GameState` (`self.CurrentState`)
    (:`NewEnumerator0`
      (`self.UpdateWarmupTimer`))
    (:`NewEnumerator1`
      (`self.UpdateGameTimer` DeltaSeconds))))

(fn `AddToHitCount`
  (bind _result (`/Engine/EditorBlueprintResources/StandardMacros.IncrementInt` (`self.HitCount`))
    (:`  `
      (set `self.HitCount` _result))))

(fn `AddToShotCount`
  (bind _result (`/Engine/EditorBlueprintResources/StandardMacros.IncrementInt` (`self.ShotCount`))
    (:`  `
      (set `self.ShotCount` _result))))

(fn `CanAfford`
  (params (Cost :type Integer))
  (returns (Result :type Boolean))
  (bind _currentpoints (`self.CurrentPoints`))
  (if (<= _currentpoints 0)
    (return false)
    (else
      (return (>= (- _currentpoints Cost) 0)))))

(fn `DisablePlayerInput`
  (bind _returnvalue (`GameplayStatics.GetPlayerPawn` 0))
  (bind _asbp_first_person_character (cast `/Game/FirstPerson/Blueprints/BP_FirstPersonCharacter` _returnvalue))
  (set `/Game/FirstPerson/Blueprints/BP_FirstPersonCharacter.FirePressed` false _asbp_first_person_character)
  (`self.DisableInput` _returnvalue null))

(fn `FormatGameTime`
  (returns (`Formatted Time` :type Text))
  (bind _survivaltime (`self.SurvivalTime`))
  (return (`|FormatText` "{Minutes}:{Seconds}" (`KismetTextLibrary.Conv_Int64ToText` (`KismetMathLibrary.FFloor64` (/ _survivaltime 60.0))) (`KismetTextLibrary.Conv_Int64ToText` (`KismetMathLibrary.FFloor64` (mod _survivaltime 60.0)) false true 2 2))))

(fn `HideWeaponPurchaseInfo`
  (`Widget.SetVisibility` (`/Game/HordeCore/Widgets/GameMode_HUD.WeaponPickupPurchase` (`self.GameModeHud`)) "Hidden"))

(fn `SaveStats`
  (bind _savedataobject (`self.SaveDataObject`))
  (bind _savedataobject_2 (`self.SaveDataObject`))
  (bind _savedataobject_3 (`self.SaveDataObject`))
  (bind _survivaltime (`self.SurvivalTime`))
  (bind _savedataobject_4 (`self.SaveDataObject`))
  (set `/Game/HordeCore/Blueprints/Game/BP_HordeGameSave.ShotsHit` (`self.HitCount`) _savedataobject_3)
  (set `/Game/HordeCore/Blueprints/Game/BP_HordeGameSave.ShotsFired` (`self.ShotCount`) _savedataobject_3)
  (set `/Game/HordeCore/Blueprints/Game/BP_HordeGameSave.LastTimeSurvived` (`self.SurvivalTime`) _savedataobject_4)
  (if (> _survivaltime (`/Game/HordeCore/Blueprints/Game/BP_HordeGameSave.BestTimeSurvived` _savedataobject_4))
    (set `/Game/HordeCore/Blueprints/Game/BP_HordeGameSave.BestTimeSurvived` _survivaltime _savedataobject_4)
    (bind _wave (`/Game/HordeCore/Blueprints/Director/BP_Director.GetCurrentWave` (`self.DirectorRef`)))
    (bind _output_get (set `/Game/HordeCore/Blueprints/Game/BP_HordeGameSave.LastWave` _wave _savedataobject_2))
    (if (> _output_get (`/Game/HordeCore/Blueprints/Game/BP_HordeGameSave.HighestWave` _savedataobject_2))
      (set `/Game/HordeCore/Blueprints/Game/BP_HordeGameSave.HighestWave` _output_get _savedataobject))
    (`GameplayStatics.SaveGameToSlot` _savedataobject "A")))

(fn `SaveTime`
  (params (SlotName :type String)))

(fn `ShowWeaponPurchaseInfo`
  (params (Cost :type Integer))
  (bind _purchasenotify (`/Game/HordeCore/Widgets/GameMode_HUD.PurchaseNotify` (`self.GameModeHud`)))
  (`Widget.SetVisibility` (`/Game/HordeCore/Widgets/GameMode_HUD.WeaponPickupPurchase` (`self.GameModeHud`)) "Visible")
  (`TextBlock.SetText` (`/Game/HordeCore/Widgets/GameMode_HUD.WeaponCost` (`self.GameModeHud`)) (`KismetTextLibrary.Conv_IntToText` Cost))
  (if (>= (`self.CurrentPoints`) Cost)
    (`Widget.SetVisibility` _purchasenotify "Visible")
    (else
      (`Widget.SetVisibility` _purchasenotify "Hidden"))))

(fn `SpendPoints`
  (params (Cost :type Integer))
  (set `self.CurrentPoints` (- (`self.CurrentPoints`) Cost))
  (`self.UpdatePointsDisplay`))

(fn `StartGame`
  (set `self.CurrentState` "NewEnumerator1")
  (`self.EnableInput` (`GameplayStatics.GetPlayerPawn` 0) (`GameplayStatics.GetPlayerController` 0))
  (`Widget.SetVisibility` (`/Game/HordeCore/Widgets/GameMode_HUD.WarmupCountdown` (`self.GameModeHud`)) "Hidden"))

(fn `UpdateGameTimer`
  (params (DeltaTime :type "Float (double-precision)"))
  (set `self.SurvivalTime` (+ DeltaTime (`self.SurvivalTime`)))
  (bind _formatted_time (`self.FormatGameTime`))
  (`TextBlock.SetText` (`/Game/HordeCore/Widgets/GameMode_HUD.TimeSurvived` (`self.GameModeHud`)) _formatted_time))

(fn `UpdatePointsDisplay`
  (`TextBlock.SetText` (`/Game/HordeCore/Widgets/GameMode_HUD.CurrentPoints` (`self.GameModeHud`)) (`KismetTextLibrary.Conv_IntToText` (`self.CurrentPoints`))))

(fn `UpdateWarmupTimer`
  (bind _returnvalue (`KismetMathLibrary.FCeil64` (- (`self.WarmupTime`) (`KismetSystemLibrary.GetGameTimeInSeconds`))))
  (`TextBlock.SetText` (`/Game/HordeCore/Widgets/GameMode_HUD.WarmupCountdown` (`self.GameModeHud`)) (`KismetTextLibrary.Conv_Int64ToText` _returnvalue))
  (if (<= _returnvalue 0)
    (`self.StartGame`)))

(fn `UserConstructionScript`)